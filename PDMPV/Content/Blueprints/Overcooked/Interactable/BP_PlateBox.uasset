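; BP_PlateBox is an interactable plate dispenser in an Overcooked-style game that hands plates to players from a stack.
; On BeginPlay it spawns a set number of BP_Plate actors, offsetting each by plate height, removing their physics and attaching them to a target component.
; GrabDrop checks whether the top plate can be grabbed, then Grab passes it to the player and removes it from the array, with no refill.
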(event EventBeginPlay
  (CallFunction|InitPlates))

(event EventGrabDrop
  (params (Player :type BP%20Character%20Object%20Reference))
  (bind _plates (Variables|Default|GetPlates))
  (if (Utilities|Array|IsNotEmpty (Variables|Default|GetPlates))
    (if (Default|CanbeGrabbed (Utilities|Array|Get(acopy) _plates (Utilities|Array|LastIndex _plates)) Player)
      (CallFunction|Grab Player))))

(event EventGrab
  (params (Player :type BP%20Character%20Object%20Reference))
  (bind _plates (Variables|Default|GetPlates))
  (bind _returnvalue (Utilities|Array|LastIndex _plates))
  (bind _output (Utilities|Array|Get(acopy) _plates _returnvalue))
  (Default|Grab _output Player)
  (Utilities|Array|RemoveItem (Variables|Default|GetPlates) _output))

(fn ConstructionScript
  (|CallParentFunction))

(fn InitPlates
  (for _index (range 1 (Variables|PlateBox|GetPlatesAmount))
    (CallFunction|AddPlate)))

(fn AddPlate
  (bind _target (Variables|Default|GetTarget))
  (bind _returnvalue (Transformation|GetWorldLocation _target))
  (bind _returnvalue_2 (Game|SpawnActorfromClass "/Game/Blueprints/Overcooked/Interactable/Kitchenware/BP_Plate.BP_Plate_C" (Math|Transform|MakeTransform (Math|Vector|MakeVector (.x _returnvalue) (.y _returnvalue) (+ (.z _returnvalue) (* (Variables|PlateBox|GetPlateHeight) (Utilities|Array|Length (Variables|Default|GetPlates)))))) "Undefined" "MultiplyWithRoot" 0 0))
  (Default|RemovePhysics _returnvalue_2)
  (Transformation|AttachComponentToComponent _returnvalue_2 (Variables|Default|GetTarget) "None" "KeepWorld" "KeepWorld" "KeepWorld" true)
  (Utilities|Array|Add (Variables|Default|GetPlates) _returnvalue_2))