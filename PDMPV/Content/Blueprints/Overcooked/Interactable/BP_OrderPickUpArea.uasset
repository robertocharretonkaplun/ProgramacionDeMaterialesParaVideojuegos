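; BP_OrderPickUpArea is an Overcooked-style interactable where players hand in filled plates.
; On GrabDrop, it checks that the player holds a non-empty BP_Plate, destroys it, and adds a plate back to a BP_PlateBox.
; It uses ConnectedPlateBox when valid, otherwise a random box from those gathered at BeginPlay.
; No order matching or scoring happens in this Blueprint.
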(event EventBeginPlay
  (Variables|PickUpArea|GetConnectedPlateBox
    (:then)
    (:else
      (bind _outactors (Actor|GetAllActorsOfClass "/Game/Blueprints/Overcooked/Interactable/BP_PlateBox.BP_PlateBox_C"))
      (Variables|PickUpArea|SetAllPlateBoxes _outactors))))

(event EventGrabDrop
  (params (Player :type BP%20Character%20Object%20Reference))
  (bind _asbp_plate (Utilities|Casting|CastToBP_Plate (.GrabbedObject (Default|GetGrabbedObject Player))))
  (if (not (Default|IsEmpty _asbp_plate))
    (Actor|DestroyActor _asbp_plate)
    (Default|AddPlate (CallFunction|GetCurrentPlateBox))))

(fn ConstructionScript)

(fn GetCurrentPlateBox
  (bind _connectedplatebox (Variables|PickUpArea|GetConnectedPlateBox)
    (:then
      (return _connectedplatebox))
    (:else
      (return (.OutItem (Utilities|Array|Random (Variables|PickUpArea|GetAllPlateBoxes)))))))