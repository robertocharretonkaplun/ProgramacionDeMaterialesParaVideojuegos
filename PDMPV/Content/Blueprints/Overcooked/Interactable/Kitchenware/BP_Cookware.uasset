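; BP_Cookware is an Overcooked-style kitchenware interactable that tracks cooking progress for the items it holds.
; The Cook event sets the cooking state and, if items are present, starts a self-calling loop that increments and debug-prints the score, then waits briefly.
; Cooking stops when the score reaches the per-item target multiplied by the item count, or when Cook disables it.
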(event Custom|UpdateCookingProgress
  (bind _result (Math|Integer|IncrementInt (Variables|Cookware|GetCookingScore))
    (:%20%20
      (Development|PrintString (Utilities|String|ToString(Integer) _result))
      (Utilities|FlowControl|Delay 0.2)
      (if (>= (Variables|Cookware|GetCookingScore) (* (Variables|Cookware|GetCookingTargetScorePerItem) (Utilities|Array|Length (Variables|Default|GetItems))))
        (Variables|Cookware|SetIsCooking false))
      (if (Variables|Cookware|GetIsCooking)
        (CallFunction|UpdateCookingProgress)))))

(event EventCook
  (params (Enable :type Boolean))
  ;[1 0.4125 0] Cook
  (bind _output_get (Variables|Cookware|SetIsCooking Enable))
  (if (and _output_get (Math|Conversions|ToBoolean(Integer) (Utilities|Array|Length (Variables|Default|GetItems))))
    (CallFunction|UpdateCookingProgress)))

(fn ConstructionScript
  (|CallParentFunction))