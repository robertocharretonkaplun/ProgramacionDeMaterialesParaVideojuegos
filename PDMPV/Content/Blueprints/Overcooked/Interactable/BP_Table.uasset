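; Interactable table for an Overcooked-style game that holds one object players can set down or pick up.
; GrabDrop branches on the player's held object: empty-handed players take the placed item, while carried items go onto a free table.
; If both are occupied, the placed item's own CanBeGrabbed and Grab handle the exchange and the slot clears.
; Place attaches keeping world transform, then moves it via MoveComponentTo.
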(event Custom|Grab
  (params (Player :type BP%20Character%20Object%20Reference))
  (Utilities|IsValid (Variables|Default|GetPlacedTarget)
    (:Is%20Valid
      (Default|Grab Player (Variables|Default|GetPlacedTarget))
      (Variables|Default|SetPlacedTarget 0))))

(event Custom|Place
  (params (ObjectToPlace :type BP%20Grabbable%20Object%20Reference) (Player :type BP%20Character%20Object%20Reference))
  (bind _output_get (Variables|Default|SetPlacedTarget ObjectToPlace))
  (Transformation|AttachComponentToComponent _output_get (Variables|Default|GetTarget) "None" "KeepWorld" "KeepWorld" "KeepWorld" true)
  (Components|MoveComponentTo (Variables|/Script/Engine.Actor|GetRootComponent (Variables|Default|GetPlacedTarget)) "0, 0, 0" "0, 0, 0" false false 0.2 false)
  (Variables|/Game/Blueprints/Overcooked/BP_Character.BP_Character_C|SetGrabbedObject Player 0))

(event EventGrabDrop
  (params (Player :type BP%20Character%20Object%20Reference))
  (bind (_returnvalue _grabbedobject) (Default|GetGrabbedObject Player))
  (if _returnvalue
    (bind _placedtarget (Variables|Default|GetPlacedTarget)
      (:then
        (if (Default|CanbeGrabbed _placedtarget Player)
          (Default|Grab (Variables|Default|GetPlacedTarget) Player)
          (Variables|Default|SetPlacedTarget 0)))
      (:else
        ;[1 0.4265 0] Place the Object to the table
        (CallFunction|Place _grabbedobject Player)))
    (else
      ;[0 1 0.06601] Grab the Object from the table
      (CallFunction|Grab Player))))

(fn ConstructionScript)