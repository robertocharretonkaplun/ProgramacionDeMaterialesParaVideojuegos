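; BP_Grabbable is an interactable object that a player can pick up and drop in an Overcooked-style game.
; GrabDrop grabs only when the player holds nothing, switching off box physics and box and mesh collision before handing itself to the player's Grab.
; Drop detaches it in world space and restores physics and collision.
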(event Custom|Drop
  ;[0.2507 1 0] Detach from actor
  (Transformation|DetachFromActor "KeepWorld" "KeepWorld" "KeepWorld")
  (CallFunction|AddPhysics))

(event Custom|Grab
  (params (Player :type BP%20Character%20Object%20Reference))
  ;[1 0.3556 0.02441] Attach to Actor
  (bind _outputpin (CallFunction|RemovePhysics Player))
  (Default|Grab _outputpin self))

(event EventGrabDrop
  (params (Player :type BP%20Character%20Object%20Reference))
  ;[0 0.7451 1] Set Object Interaction
  (if (CallFunction|CanbeGrabbed Player)
    (CallFunction|Grab Player)))

(fn ConstructionScript)

(fn CanbeGrabbed
  (params (Player :type BP%20Character%20Object%20Reference))
  (return (not (.ReturnValue (Default|GetGrabbedObject Player)))))

(fn RemovePhysics
  (params (InputPin :type BP%20Character%20Object%20Reference))
  (bind _box (Variables|Default|GetBox))
  (Physics|SetSimulatePhysics _box false)
  (Collision|SetCollisionEnabled _box "NoCollision")
  (Collision|SetCollisionEnabled (Variables|Default|GetMesh) "NoCollision")
  (return InputPin))

(fn AddPhysics
  (bind _box (Variables|Default|GetBox))
  (Physics|SetSimulatePhysics _box true)
  (Collision|SetCollisionEnabled _box "QueryAndPhysics")
  (Collision|SetCollisionEnabled (Variables|Default|GetMesh) "QueryAndPhysics"))