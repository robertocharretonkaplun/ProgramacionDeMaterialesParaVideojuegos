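; BP_FoodBox is an interactable food crate in an Overcooked-style kitchen that dispenses food items to players.
; With a placed object on it, it runs the parent grab/drop logic if that object can be grabbed.
; When empty, it runs the parent logic if the player holds something, otherwise spawns a BP_FoodItem at its transform and immediately hands it to the player via GrabDrop.
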(event EventGrabDrop
  (params (Player :type BP%20Character%20Object%20Reference))
  (bind _placedtarget (Variables|Default|GetPlacedTarget)
    (:then
      (if (Default|CanbeGrabbed _placedtarget Player)
        (|CallParentFunction Player :!label _label)))
    (:else
      (if (.ReturnValue (Default|GetGrabbedObject Player))
        (goto _label)
        (else
          (bind _returnvalue (Game|SpawnActorfromClass "/Game/Blueprints/Overcooked/Interactable/BP_FoodItem.BP_FoodItem_C" (Transformation|GetActorTransform) "Undefined" "MultiplyWithRoot" 0 true 0))
          (Default|GrabDrop _returnvalue Player))))))

(fn ConstructionScript
  (|CallParentFunction))