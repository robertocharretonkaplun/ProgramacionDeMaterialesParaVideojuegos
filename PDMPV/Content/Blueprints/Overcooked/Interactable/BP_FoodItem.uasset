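; Food ingredient actor for an Overcooked-style kitchen that players can pick up and, if flagged sliceable, slice.
; A Raw, Slicing or Sliced state, starting at Raw, swaps the mesh material and blocks slicing once sliced.
; Grabbing removes physics, then puts the item in an empty-handed player's grip or passes it to the held object through an AddItem message.
; The grab check allows only empty hands or a held dish with free space.
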(event Custom|SetState
  (params (State :type BPE_FoodItemStates%20Enum :default "NewEnumerator0"))
  (bind _output_get (Variables|Default|SetState State))
  (Rendering|Material|SetMaterial (Variables|Character|GetMesh) 0 (Utilities|Select :Index _output_get :NewEnumerator0 "/Game/Materials/BaseColor/M_Raw.M_Raw" :NewEnumerator1 "/Game/Materials/BaseColor/m_Slicing.m_Slicing" :NewEnumerator2 "/Game/Materials/BaseColor/M_Sliced.M_Sliced")))

(event EventBeginPlay
  (CallFunction|SetState "NewEnumerator0"))

(event Collision|EventActorBeginOverlap
  (params (OtherActor :type Actor%20Object%20Reference)))

(event EventTick
  (params (DeltaSeconds :type Float%20%28single-precision%29)))

(event EventGrab
  (params (Player :type BP%20Character%20Object%20Reference))
  (bind (_returnvalue _grabbedobject) (Default|GetGrabbedObject Player))
  (bind _self self)
  (CallFunction|RemovePhysics)
  (if _returnvalue
    (Class|BPIDish|AddItem(Message) _grabbedobject _self)
    (else
      (Default|Grab Player _self))))

(fn ConstructionScript
  (|CallParentFunction))

(fn CanbeSliced
  (return (and (Variables|Default|GetIsSlicable) (Utilities|Select :Index (Variables|Default|GetState) :NewEnumerator0 true :NewEnumerator1 true :NewEnumerator2 false))))

(fn CanbeGrabbed
  (params (Player :type BP%20Character%20Object%20Reference))
  (bind (_returnvalue _grabbedobject) (Default|GetGrabbedObject Player))
  (if (not _returnvalue)
    (return true)
    (else
      (bind _asbp_kitchenware (Utilities|Casting|CastToBP_Dish _grabbedobject)
        (:then
          (return (Default|HasPlace _asbp_kitchenware)))
        (:CastFailed
          (return false))))))